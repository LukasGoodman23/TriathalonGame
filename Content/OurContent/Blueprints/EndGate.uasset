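; EndGate is a finish-line gate that times a run and prints the elapsed time when something reaches it.
; Activate starts a timer loop that adds a tenth of a second after each 0.1 second delay while IsActive is set.
; Any overlap with the Box calls Finish, which stops the timer and prints the final time to screen.
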(event OnComponentBeginOverlap(Box)
  (params (OverlappedComponent :type Primitive%20Component%20Object%20Reference) (OtherActor :type Actor%20Object%20Reference) (OtherComp :type Primitive%20Component%20Object%20Reference) (OtherBodyIndex :type Integer) (bFromSweep :type Boolean) (SweepResult :type Hit%20Result%20Structure%20%28by%20ref%29))
  (CallFunction|Finish))

(event Custom|Activate
  (bind _output_get (Variables|Default|Setis_Active true))
  ;[0 0 0] Timer
  (if _output_get :!label _label
    (Utilities|FlowControl|Delay 0.1)
    (Variables|Default|SetTime (+ (Variables|Default|GetTime) 0.1))
    (goto _label)))

(event Custom|Finish
  ;[0 0 0] Prints out final time
  (if (Variables|Default|Getis_Active)
    (Variables|Default|Setis_Active false)
    (Development|PrintString (Utilities|String|ToString(Float) (Variables|Default|GetTime)))))

(fn ConstructionScript)
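; PositionPath is a Blueprint data holder for a path of positions, each paired with a distance offset, with no active event or construction logic.
; It stores the path in two index-matched arrays, PositionArray and DistanceFromPos.
; Getter functions return a position, an offset or both for a given index, plus the position count and a fixed default offset.
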(event EventBeginPlay)

(event Collision|EventActorBeginOverlap
  (params (OtherActor :type Actor%20Object%20Reference)))

(event EventTick
  (params (DeltaSeconds :type Float%20%28single-precision%29)))

(fn ConstructionScript)

(fn GetPositionfromIndex
  (params (Index%20Value :type Integer))
  (return (Utilities|Array|Get(acopy) (Variables|Default|GetPositionArray) Index%20Value)))

(fn GetLengthOfArrays
  (return (Utilities|Array|Length (Variables|Default|GetPositionArray))))

(fn GetOffsetfromIndex
  (params (Area%20Index :type Integer))
  (return (Utilities|Array|Get(acopy) (Variables|Default|GetDistanceFromPos) Area%20Index)))

(fn GetDefaultOffset
  (return (Math|Float|MakeLiteralFloat 1e+02)))

(fn GetBothfromIndex
  (params (Input :type Integer))
  (return (Utilities|Array|Get(acopy) (Variables|Default|GetPositionArray) Input) (Utilities|Array|Get(acopy) (Variables|Default|GetDistanceFromPos) Input)))
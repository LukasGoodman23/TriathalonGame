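; WaveSim simulates a water surface with a grid of blue, collision-free cubes.
; The construction script builds the grid as nested WaterBody arrays of mesh components.
; From BeginPlay, a delay loop steps a wrapping Time counter and sets each cube's Z from two summed, phase-shifted GetHeight samples, one per grid axis.
; GetHeight contains a scaled cosine formula, but it appears unconnected.
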(event EventBeginPlay
  (CallFunction|SetWaveHeights :!label _label)
  (Utilities|FlowControl|Delay 0.025)
  (Variables|Default|SetTime (+ (Variables|Default|GetTime) 1.0))
  (if (>= (Variables|Default|GetTime) 256.0)
    (Variables|Default|SetTime 0.0)
    (goto _label)
    (else
      (goto _label))))

(fn ConstructionScript
  (bind _cubesize (Variables|Default|GetCubeSize))
  (for _index (range 0 (- (Variables|Default|GetWaveWidthInCubes) 1))
    (for _index_2 (range 0 (- (Variables|Default|GetWaveLengthInCubes) 1))
      (if (== _index_2 0)
        (Utilities|Array|Add (Variables|Default|GetWaterBody) (Utilities|Struct|MakeStruct_Wave)))
      (bind _returnvalue (AddComponent|AddStaticMeshComponent false (Math|Transform|MakeTransform (Math|Vector|MakeVector (* _index _cubesize) (* _index_2 _cubesize) (.z (Transformation|GetWorldLocation (Variables|Default|GetDefaultSceneRoot)))) "0, 0, 0" (Math|Conversions|ToVector(Float) (/ (Variables|Default|GetCubeSize) 1e+02)))))
      (Components|StaticMesh|SetStaticMesh _returnvalue "/Game/LevelPrototyping/Meshes/SM_Cube.SM_Cube")
      (Collision|SetCollisionEnabled _returnvalue "NoCollision")
      (Rendering|Material|SetMaterial _returnvalue 0 "/Game/LevelPrototyping/Materials/MI_Solid_Blue.MI_Solid_Blue")
      (Utilities|Array|Add (Utilities|Struct|BreakStruct_Wave (Utilities|Array|Get(acopy) (Variables|Default|GetWaterBody) _index)) _returnvalue))))

(fn SetWaveHeights
  (for (_array_element _array_index) (Variables|Default|GetWaterBody)
    (for (_array_element_2 _array_index_2) (Utilities|Struct|BreakStruct_Wave _array_element)
      (Utilities|IsValid _array_element_2
        (:Is%20Valid
          (Transformation|SetWorldLocation _array_element_2 (Math|Vector|MakeVector (.x (Transformation|GetWorldLocation _array_element_2)) (.y (Transformation|GetWorldLocation _array_element_2)) (+ (.z (Transformation|GetWorldLocation (Variables|Default|GetDefaultSceneRoot))) (+ (Utilities|GetHeight (- (Variables|Default|GetTime) (* _array_index_2 32))) (Utilities|GetHeight (- (Variables|Default|GetTime) (* _array_index 24)))))) false false))))))